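; BP_BoxTriggerTest3 is a functional test that checks a trigger box changes the character's health to an expected value.
; On prepare, it places the character a short distance before the TriggerBox along the X axis.
; Each tick it drives the character forward and succeeds once its health equals EndStateHealth.
; The graph has no explicit failure branch.
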(event EventPrepareTest
  (Transformation|SetActorLocation (Variables|Default|GetCharacter) (- (Transformation|GetActorLocation (Variables|Default|GetTriggerBox)) "500.000000,0.000000,0.000000") false false))

(event EventStartTest)

(event EventTick
  (params (DeltaSeconds :type Float%20%28single-precision%29))
  (bind _character (Variables|Default|GetCharacter))
  (Pawn|Input|AddMovementInput _character (Transformation|GetActorForwardVector _character) 1.0 false)
  (bind _returnvalue (Class|ExperisChallengeCharacter|GetHealth (Variables|Default|GetCharacter)))
  (if (== (Variables|Default|GetEndStateHealth) _returnvalue)
    (Class|FunctionalTest|FinishTest "Succeeded" "It Worked")))

(fn ConstructionScript)