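; Functional test that checks a trigger box changes the third-person character's Health as expected.
; PrepareTest places the character short of the TriggerBox along X and binds to its OnPlayerDied event.
; Tick walks the character forward and passes once Health equals EndStateHealth.
; When that target is zero, it also requires OnPlayerDied to have fired, failing otherwise.
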(event Custom|PlayerDiedFired
  (bind _output_get (Variables|Default|SetDidPlayerDiedFire true))
  (Class|FunctionalTest|AssertTrue _output_get))

(event EventPrepareTest
  (Transformation|SetActorLocation (Variables|Default|GetCharacter) (- (Transformation|GetActorLocation (Variables|Default|GetTriggerBox)) "500.000000,0.000000,0.000000") false false)
  (bind _asbp_third_person_character (Utilities|Casting|CastToBP_ThirdPersonCharacter (Variables|Default|GetCharacter)))
  (EventDispatchers|BindEventtoOnPlayerDied _asbp_third_person_character (delegate Custom|PlayerDiedFired)))

(event EventStartTest)

(event EventTick
  (params (DeltaSeconds :type Float%20%28single-precision%29))
  (bind _character (Variables|Default|GetCharacter))
  (Pawn|Input|AddMovementInput _character (Transformation|GetActorForwardVector _character) 1.0 false)
  (if (== (Variables|/Script/ExperisChallenge.ExperisChallengeCharacter|GetHealth (Variables|Default|GetCharacter)) (Variables|Default|GetEndStateHealth))
    (if (== (Variables|Default|GetEndStateHealth) 0)
      ;[1 1 1] Check if PlayerDied fired
      (if (Variables|Default|GetDidPlayerDiedFire)
        (Class|FunctionalTest|FinishTest "Succeeded" "Test Passed")
        (else
          (Class|FunctionalTest|FinishTest "Failed" "PlyerDided did not fire")))
      (else
        (Class|FunctionalTest|FinishTest "Succeeded" "Test Passed")))))

(fn ConstructionScript)