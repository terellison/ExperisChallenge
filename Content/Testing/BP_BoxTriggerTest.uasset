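; BP_BoxTriggerTest is a functional test that passes once the Character's health changes, presumably from a trigger box.
; StartTest sets health to 20, stores it, then polls GetHealth in a while loop until it differs and finishes as Succeeded.
; The loop has no delay or failure branch.
; The movement input node that references TriggerBox1's location is never executed, so the test itself does not move the Character.
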(event EventPrepareTest)

(event EventStartTest
  (bind _character (Variables|Default|GetCharacter))
  (Class|ExperisChallengeCharacter|SetHealth _character 20)
  (bind _returnvalue (Class|ExperisChallengeCharacter|GetHealth _character))
  (Variables|Default|SetPreviousHealth _returnvalue)
  (while (== (Variables|Default|GetPreviousHealth) (stale _returnvalue_2))
    (bind _returnvalue_2 (Class|ExperisChallengeCharacter|GetHealth _character)))
  (Class|FunctionalTest|FinishTest "Succeeded" "It Worked"))

(event EventTick
  (params (DeltaSeconds :type Float%20%28single-precision%29)))

(fn ConstructionScript)